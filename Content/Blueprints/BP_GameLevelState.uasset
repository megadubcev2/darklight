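; Level state Blueprint that lets the player toggle a room light switch with K, changing vision mode and sun brightness to match.
; BeginPlay links the first found switch to the first found bulb, lights it and binds character key and switch proximity events.
; When the player is near, ToggleLight flips the switch and passes its inverted state to SetDarkMode.
; SetDarkMode swaps the character's night-vision variant and the directional light's intensity.
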(event `self.ReceiveBeginPlay`
  (bind _asbp_first_person_character (cast `/Game/FirstPerson/Blueprints/BP_FirstPersonCharacter` (`GameplayStatics.GetPlayerCharacter` 0)))
  (add `/Game/FirstPerson/Blueprints/BP_FirstPersonCharacter.OnPressedK` _asbp_first_person_character (`|CreateDelegate` :!event `PlayerPressedK`))
  (bind _outactors (`GameplayStatics.GetAllActorsOfClass` "/Game/Blueprints/BP_LightingBulb.BP_LightingBulb_C"))
  (bind _outactors_2 (`GameplayStatics.GetAllActorsOfClass` "/Game/Blueprints/BP_LightSwitch.BP_LightSwitch_C"))
  (bind _output_get (set `self.LightSwitch` (`|GetArrayItem` _outactors_2)))
  (bind _output_get_2 (set `/Game/Blueprints/BP_LightSwitch.LightingBulb` (`|GetArrayItem` _outactors) _output_get))
  (`/Game/Blueprints/BP_LightingBulb.TurnLight` _output_get_2)
  (add `/Game/Blueprints/BP_LightSwitch.OnComponentBecomeNear` _output_get (`|CreateDelegate` :!event `ComponentNearLightSwitch`))
  (`self.SetDarkMode` false))

(event `PlayerPressedK`
  (if (`/Game/Blueprints/BP_LightSwitch.IsPersonNear` (`self.LightSwitch`))
    (`self.ToggleLight`)
    (`KismetSystemLibrary.PrintText` "Hello")))

(event `ComponentNearLightSwitch`
  (params (LightSwitch :type "/Game/Blueprints/BP_LightSwitch Object Reference") (Actor :type "Actor Object Reference"))
  (cast `/Game/FirstPerson/Blueprints/BP_FirstPersonCharacter` Actor)
  (set `/Game/Blueprints/BP_LightSwitch.IsPersonNear` true LightSwitch))

(event `ComponentFarLightSwitch`
  (params (LightSwitch :type "/Game/Blueprints/BP_LightSwitch Object Reference") (Actor :type "Actor Object Reference"))
  (cast `/Game/FirstPerson/Blueprints/BP_FirstPersonCharacter` Actor)
  (set `/Game/Blueprints/BP_LightSwitch.IsPersonNear` false LightSwitch))

(fn `SetDarkMode`
  (params (IsDarkMode :type Boolean))
  (if IsDarkMode
    (bind _asbp_first_person_character (cast `/Game/FirstPerson/Blueprints/BP_FirstPersonCharacter` (`GameplayStatics.GetPlayerCharacter` 0)))
    (`/Game/FirstPerson/Blueprints/BP_FirstPersonCharacter.TurnNightVision` _asbp_first_person_character)
    (bind _outactors (`GameplayStatics.GetAllActorsOfClass` "/Script/Engine.DirectionalLight"))
    (`LightComponent.SetIntensity` (`Light.LightComponent` (`|GetArrayItem` _outactors)) 5.0)
    (`KismetSystemLibrary.PrintText` "day")
    (else
      (bind _asbp_first_person_character_2 (cast `/Game/FirstPerson/Blueprints/BP_FirstPersonCharacter` (`GameplayStatics.GetPlayerCharacter` 0)))
      (`/Game/FirstPerson/Blueprints/BP_FirstPersonCharacter.TurnNightVisionLight` _asbp_first_person_character_2)
      (bind _outactors_2 (`GameplayStatics.GetAllActorsOfClass` "/Script/Engine.DirectionalLight"))
      (`LightComponent.SetIntensity` (`Light.LightComponent` (`|GetArrayItem` _outactors_2)) 0.01)
      (`KismetSystemLibrary.PrintText` "day"))))

(fn `ToggleLight`
  (bind _lightswitch (`self.LightSwitch`))
  (`/Game/Blueprints/BP_LightSwitch.ToggleLight` _lightswitch)
  (bind _isturnin (`/Game/Blueprints/BP_LightSwitch.IsTurnIn` _lightswitch))
  (`self.SetDarkMode` (not _isturnin)))

(fn `UserConstructionScript`)