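; BP_LightSwitch is a light switch actor that turns a referenced LightingBulb on or off.
; Box overlap begin and end events pass the switch and overlapping actor to become-near and become-far calls.
; ToggleLight flips the IsTurnOn state and applies it through SetTurn, which calls the bulb's on or off function.
; InitBulb applies the current state to the bulb, though BeginPlay in this file does not call it.
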(event `self.ReceiveBeginPlay`)

(event `self.Box.OnComponentBeginOverlap`
  (params (OverlappedComponent :type "PrimitiveComponent Object Reference") (OtherActor :type "Actor Object Reference") (OtherComp :type "PrimitiveComponent Object Reference") (OtherBodyIndex :type Integer) (bFromSweep :type Boolean) (SweepResult :type "HitResult Structure (by ref)"))
  (`self.OnComponentBecomeNear` self OtherActor))

(event `self.Box.OnComponentEndOverlap`
  (params (OverlappedComponent :type "PrimitiveComponent Object Reference") (OtherActor :type "Actor Object Reference") (OtherComp :type "PrimitiveComponent Object Reference") (OtherBodyIndex :type Integer))
  (`self.OnComponentBecomeFar` self OtherActor))

(fn `InitBulb`
  (`self.Set Turn` (`self.IsTurnOn`)))

(fn `Set Turn`
  (params (IsTurnOn :type Boolean))
  (bind _lightingbulb (`self.LightingBulb`))
  (if IsTurnOn
    (`/Game/Blueprints/BP_LightingBulb.TurnOnLight` _lightingbulb)
    (else
      (`/Game/Blueprints/BP_LightingBulb.OffLight` _lightingbulb))))

(fn `ToggleLight`
  (bind _output_get (set `self.IsTurnOn` (not (`self.IsTurnOn`))))
  (`self.Set Turn` _output_get))

(fn `UserConstructionScript`)