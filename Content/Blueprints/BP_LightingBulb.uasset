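; BP_LightingBulb is a light bulb actor that can be switched on and off.
; ToggleLight checks PointLight visibility and calls TurnOnLight or OffLight, which show or hide the light and swap the bulb mesh between lit and base materials.
; BeginPlay sets two intensity values.
; Disconnected sphere-trace debug graphs that would hide the light remain in the EventGraph but never run.
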(event `self.ReceiveBeginPlay`
  (set `self.IntensityLight` 8000.0)
  (set `self.Intensity` 1600.0))

(event `self.ReceiveTick`
  (params (DeltaSeconds :type "Float (single-precision)")))

(fn `OffLight`
  (`SceneComponent.SetVisibility` (`self.PointLight`) false false)
  (`PrimitiveComponent.SetMaterial` (`self.light_bulb_fbx_fbx_bulb`) 0 "/Game/FPWeapon/Materials/BaseMaterial.BaseMaterial"))

(fn `ToggleLight`
  (if (`SceneComponent.IsVisible` (`self.PointLight`))
    (`self.OffLight`)
    (else
      (`self.TurnOnLight`))))

(fn `TurnOnLight`
  (`SceneComponent.SetVisibility` (`self.PointLight`) true false)
  (`PrimitiveComponent.SetMaterial` (`self.light_bulb_fbx_fbx_bulb`) 0 "/Game/StaticMeshes/source/material_3.material_3"))

(fn `UserConstructionScript`)