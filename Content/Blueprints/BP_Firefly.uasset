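; BP_Firefly is a firefly actor that bobs vertically and holds a text string loaded from a data table.
; Each Tick moves it along the normalized Direction by Speed and delta time, without sweep.
; A Delay chained to Tick feeds a FlipFlop that alternates Direction between down and up at a fixed interval.
; On BeginPlay it looks up TextKey in DT_FireflyText and stores the row's Text.
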(event `self.ReceiveTick`
  (params (DeltaSeconds :type "Float (single-precision)"))
  ;[1 1 1] Движение
  (`self.K2_SetActorTransform` (`KismetMathLibrary.MakeTransform` (+ (* (`KismetMathLibrary.Normal` (`self.direction`)) (* (`GameplayStatics.GetWorldDeltaSeconds`) (`self.speed`))) (.location (`SceneComponent.K2_GetComponentToWorld` (`self.DefaultSceneRoot`)))) (.rotation (`SceneComponent.K2_GetComponentToWorld` (`self.DefaultSceneRoot`))) (.scale (`SceneComponent.K2_GetComponentToWorld` (`self.DefaultSceneRoot`)))))
  (`KismetSystemLibrary.Delay` 1.5)
  (`/Engine/EditorBlueprintResources/StandardMacros.FlipFlop`
    (:`A`
      (set `self.direction` (0.0 0.0 -10.0)))
    (:`B`
      (set `self.direction` (0.0 0.0 10.0)))))

(event `self.ReceiveBeginPlay`
  ;[1 1 1] Найти текст
  (bind _returnvalue (`|GetDataTableRow` "/Game/DataTables/DT_FireflyText.DT_FireflyText" (`KismetStringLibrary.Conv_StringToName` (`self.textKey`)))
    (:`then`
      (set `self.text` (`.text_4_835306EA4C5C242D3054CDB105B4DC30` (break `/Game/DataTables/S_Text` _returnvalue))))))

(fn `UserConstructionScript`)